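; Weapon Blueprint for a shotgun that handles firing, reloading and aim-down-sights zoom through components.
; Fire checks the Ammo and FireModeShotgun components, then fires, plays a camera shake, consumes ammo and starts the recoil timer.
; Reload is delegated to Ammo, and zoom toggles the given camera through the Zoom component with scope settings enabled.
; On BeginPlay, the Recoil component receives the player pawn.
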(event EventOnZoomEvent
  (params (Camera :type Camera%20Component%20Object%20Reference))
  (Class|Zoom|ZoomToggle (Variables|Default|GetZoom) Camera 4.0 5.0 true))

(event EventBeginPlay
  ;[1 1 1] Set Pawn for Recoil
  (Class|Recoil|SetPawn (Variables|Default|GetRecoil) (Game|Player|GetPlayerPawn 0)))

(event EventOnFireEvent
  (params (Pawn :type Pawn%20Object%20Reference))
  (bind _returnvalue (Class|Ammo|CheckAmmo (Variables|Default|GetAmmo)))
  (if (and _returnvalue (Variables|/Script/WeaponSystem_Team7.FireMode_Shotgun|GetbCanFire (Variables|Default|GetFireMode_Shotgun)))
    (Class|FireModeShotgun|Fire (Variables|Default|GetFireMode_Shotgun))
    (Class|Weapon|WeaponCameraShake)
    (Class|Ammo|UseAmmo (Variables|Default|GetAmmo))
    (Class|Recoil|StartRecoilTimer (Variables|Default|GetRecoil))))

(event EventOnReloadEvent
  (Class|Ammo|Reload (Variables|Default|GetAmmo)))

(fn ConstructionScript)