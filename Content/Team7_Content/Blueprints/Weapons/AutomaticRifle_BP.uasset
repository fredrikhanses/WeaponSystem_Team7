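; Automatic rifle weapon Blueprint that fires continuously while the fire input is held and supports reload and scopeless zoom.
; Input events delegate to Fire, Zoom and Ammo components, with Fire receiving the fire mode, SFX, VFX, Ammo, Recoil and KickBack components on each trigger pull.
; BeginPlay binds Recoil to the player pawn with a camera shake and KickBack to the player character with a first-person fire montage.
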(event EventOnFireEvent
  (Class|Fire|ToggleAutofire (Variables|Default|GetFire) true)
  (Class|Fire|OnFire (Variables|Default|GetFire) (Utilities|Array|MakeArray (Variables|Default|GetFireMode) (Variables|Default|GetSFX) (Variables|Default|GetVFX) (Variables|Default|GetAmmo) (Variables|Default|GetRecoil) (Variables|Default|GetKickBack))))

(event EventOnZoomEvent
  (params (Camera :type Camera%20Component%20Object%20Reference))
  (Class|Zoom|ZoomToggle (Variables|Default|GetZoom) Camera 0.0 false))

(event EventOnReloadEvent
  (Class|Ammo|Reload (Variables|Default|GetAmmo)))

(event EventOnReleaseEvent
  (Class|Fire|ToggleAutofire (Variables|Default|GetFire) false))

(event EventBeginPlay
  (bind _kickback (Variables|Default|GetKickBack))
  (Class|Recoil|SetPawn (Variables|Default|GetRecoil) (Game|Player|GetPlayerPawn 0))
  (Class|Recoil|SetCameraShake (Variables|Default|GetRecoil) "/Game/Team7_Content/Blueprints/AutomaticWeaponShake_BP.AutomaticWeaponShake_BP_C")
  (Class|KickBack|SetAnimation _kickback "/Game/FirstPerson/Animations/FirstPersonFire_Montage.FirstPersonFire_Montage")
  (Class|KickBack|SetCharacter _kickback (Game|GetPlayerCharacter 0)))

(fn ConstructionScript)