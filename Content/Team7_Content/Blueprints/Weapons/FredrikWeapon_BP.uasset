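; Weapon Blueprint for an FPS gun that handles fire, release, reload and zoom events by delegating to components.
; On BeginPlay it hooks Recoil to player pawn 0 with a camera shake and toggles a red gun skin through SkinToggle.
; Firing enables autofire and, if Ammo covers the burst count, passes fire mode, SFX, VFX, ammo and recoil to Fire.
; Zoom toggles without a scope.
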(event EventOnZoomEvent
  (params (Camera :type Camera%20Component%20Object%20Reference))
  (Class|Zoom|ZoomToggle (Variables|Default|GetZoom) Camera 4.0 false))

(event EventOnReleaseEvent
  (Variables|/Script/WeaponSystem_Team7.Fire|SetbAutofire (Variables|Default|GetFire) false))

(event EventBeginPlay
  (bind _recoil (Variables|Default|GetRecoil))
  (bind _skintoggle (Variables|Default|GetSkinToggle))
  ;[1 1 1] Set Pawn and CameraShake for Recoil
  (Class|Recoil|SetPawn _recoil (Game|Player|GetPlayerPawn 0))
  (Class|Recoil|SetCameraShake _recoil)
  (Class|SkinToggle|SetMaterial _skintoggle "/Game/Team7_Content/Materials/M_FPGun_Red.M_FPGun_Red")
  (Class|SkinToggle|Toggle _skintoggle))

(event EventOnFireEvent
  (bind _ammo (Variables|Default|GetAmmo))
  (Variables|/Script/WeaponSystem_Team7.Fire|SetbAutofire (Variables|Default|GetFire) true)
  (bind _returnvalue (Class|Ammo|CheckAmmo _ammo))
  (if (and _returnvalue (>= (Variables|/Script/WeaponSystem_Team7.Ammo|GetCurrentAmmo _ammo) (Variables|/Script/WeaponSystem_Team7.Fire|GetBurstCount (Variables|Default|GetFire))))
    (Class|Fire|OnFire (Variables|Default|GetFire) (Utilities|Array|MakeArray (Variables|Default|GetFireMode) (Variables|Default|GetSFX) (Variables|Default|GetVFX) (Variables|Default|GetAmmo) (Variables|Default|GetRecoil)))))

(event EventOnReloadEvent
  (Class|Ammo|Reload (Variables|Default|GetAmmo)))

(fn ConstructionScript)