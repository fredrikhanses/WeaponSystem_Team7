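; Dual-firemode shotgun weapon Blueprint with primary and secondary fire (single / burst) and reload.
; Each trigger passes its own firemode, recoil and kickback components, plus shared ammo, VFX and SFX, to a fire component.
; BeginPlay registers ammo and UI color components and binds both recoil and kickback sets to player 0 with a shotgun camera shake and first-person fire montage.
; Reload delegates to the ammo component.
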(event EventOnPrimaryPressed
  ;[0 0.4336 1] Dual firemode Shotgun (Single / burst)
  ;;[1 1 1] Primary fire
  (Class|Fire|OnFire (Variables|Default|GetPrimaryFire) (Utilities|Array|MakeArray (Variables|Default|GetPrimaryFireMode) (Variables|Default|GetPrimaryRecoil) (Variables|Default|GetAmmo) (Variables|Default|GetVFX) (Variables|Default|GetSFX) (Variables|Default|GetPrimaryKickBack))))

(event EventBeginPlay
  (bind _returnvalue (Game|GetPlayerCharacter 0))
  (bind _returnvalue_2 (Game|Player|GetPlayerPawn 0))
  (bind _secondarykickback (Variables|Default|GetSecondaryKickBack))
  (bind _primarykickback (Variables|Default|GetPrimaryKickBack))
  ;[0 0.4336 1] Dual firemode Shotgun (Single / burst)
  ;;[1 1 1] Initiate Properties
  (Class|Weapon|SetAmmoComponent (Variables|Default|GetAmmo))
  (Class|Recoil|SetPawn (Variables|Default|GetPrimaryRecoil) _returnvalue_2)
  (Class|Recoil|SetPawn (Variables|Default|GetSecondaryRecoil) _returnvalue_2)
  (Class|Recoil|SetCameraShake (Variables|Default|GetPrimaryRecoil) "/Game/Team7_Content/Blueprints/CameraShake/ShotgunShake_BP.ShotgunShake_BP_C")
  (Class|Recoil|SetCameraShake (Variables|Default|GetSecondaryRecoil) "/Game/Team7_Content/Blueprints/CameraShake/ShotgunShake_BP.ShotgunShake_BP_C")
  (Class|KickBack|SetAnimation _primarykickback "/Game/FirstPerson/Animations/FirstPersonFire_Montage.FirstPersonFire_Montage")
  (Class|KickBack|SetCharacter _primarykickback _returnvalue)
  (Class|KickBack|SetAnimation _secondarykickback "/Game/FirstPerson/Animations/FirstPersonFire_Montage.FirstPersonFire_Montage")
  (Class|KickBack|SetCharacter _secondarykickback _returnvalue)
  (Class|Weapon|SetUIColorComponent (Variables|Default|GetUIColor)))

(event EventOnReload
  ;[0 0.4336 1] Dual firemode Shotgun (Single / burst)
  ;;[1 1 1] Reload
  (Class|Ammo|Reload (Variables|Default|GetAmmo)))

(event EventOnSecondary
  (params (Camera :type Camera%20Component%20Object%20Reference))
  ;[0 0.4336 1] Dual firemode Shotgun (Single / burst)
  ;;[1 1 1] Secondary Fire
  (Class|Fire|OnFire (Variables|Default|GetSecondaryFire) (Utilities|Array|MakeArray (Variables|Default|GetSecondaryFireMode) (Variables|Default|GetSecondaryRecoil) (Variables|Default|GetAmmo) (Variables|Default|GetVFX) (Variables|Default|GetSFX) (Variables|Default|GetSecondaryKickBack))))

(fn ConstructionScript)