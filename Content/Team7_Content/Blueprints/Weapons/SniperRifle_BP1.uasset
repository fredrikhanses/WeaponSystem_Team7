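; Sniper rifle weapon Blueprint with primary fire, scoped secondary zoom and reloading, built from components.
; Primary fire passes fire mode, recoil, ammo, VFX, SFX and kickback components to the PrimaryFire component's OnFire.
; Secondary input toggles a scope zoom on the passed camera, and reload is delegated to the Ammo component.
; BeginPlay registers ammo and binds recoil camera shake and kickback animation to player zero's pawn and character.
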(event EventOnPrimaryPressed
  ;[0.3532 1 0.2572] Sniper Rifle
  ;;[1 1 1] Primary fire
  (Class|Fire|OnFire (Variables|Default|GetPrimaryFire) (Utilities|Array|MakeArray (Variables|Default|GetPrimaryFireMode) (Variables|Default|GetPrimaryRecoil) (Variables|Default|GetAmmo) (Variables|Default|GetVFX) (Variables|Default|GetSFX) (Variables|Default|GetPrimaryKickBack))))

(event EventBeginPlay
  (bind _primarykickback (Variables|Default|GetPrimaryKickBack))
  ;[0.3532 1 0.2572] Sniper Rifle
  ;;[1 1 1] Initiate Properties
  (Class|Weapon|SetAmmoComponent (Variables|Default|GetAmmo))
  (Class|Recoil|SetPawn (Variables|Default|GetPrimaryRecoil) (Game|Player|GetPlayerPawn 0))
  (Class|Recoil|SetCameraShake (Variables|Default|GetPrimaryRecoil) "/Game/Team7_Content/Blueprints/CameraShake/AutomaticWeaponShake_BP.AutomaticWeaponShake_BP_C")
  (Class|KickBack|SetAnimation _primarykickback "/Game/FirstPerson/Animations/FirstPersonFire_Montage.FirstPersonFire_Montage")
  (Class|KickBack|SetCharacter _primarykickback (Game|GetPlayerCharacter 0)))

(event EventOnReload
  ;[0.3532 1 0.2572] Sniper Rifle
  ;;[1 1 1] Reload
  (Class|Ammo|Reload (Variables|Default|GetAmmo)))

(event EventOnSecondary
  (params (Camera :type Camera%20Component%20Object%20Reference))
  ;[0.3532 1 0.2572] Sniper Rifle
  ;;[1 1 1] Zoom
  (Class|Zoom|ZoomToggle (Variables|Default|GetZoom) Camera 6.0 true))

(fn ConstructionScript)