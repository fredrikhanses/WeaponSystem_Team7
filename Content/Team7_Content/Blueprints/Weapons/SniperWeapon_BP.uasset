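; Sniper weapon Blueprint that wires zoom, fire and reload events to its components.
; On BeginPlay it registers Ammo, gives Recoil the first player's pawn and a camera shake, and applies a blue skin through SkinToggle.
; Firing requires an ammo check and enough rounds for the burst, then passes FireMode, SFX, VFX, Ammo and Recoil to Fire.
; Zoom toggles a fixed-magnification scope, and reload delegates to Ammo.
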(event EventBeginPlay
  (bind _recoil (Variables|Default|GetRecoil))
  (bind _skintoggle (Variables|Default|GetSkinToggle))
  (Class|Weapon|SetAmmoComponent (Variables|Default|GetAmmo))
  (Class|Recoil|SetPawn _recoil (Game|Player|GetPlayerPawn 0))
  (Class|Recoil|SetCameraShake _recoil "/Game/Team7_Content/Blueprints/WeaponCameraShake_BP.WeaponCameraShake_BP_C")
  (Class|SkinToggle|SetMaterial _skintoggle "/Game/Team7_Content/Materials/M_FPGun_Blue.M_FPGun_Blue")
  (Class|SkinToggle|Toggle _skintoggle))

(event EventOnZoomEvent
  (params (Camera :type Camera%20Component%20Object%20Reference))
  (Class|Zoom|ZoomToggle (Variables|Default|GetZoom) Camera 4.0 true))

(event EventOnFireEvent
  (bind _ammo (Variables|Default|GetAmmo))
  (bind _returnvalue (Class|Ammo|CheckAmmo _ammo))
  (if (and _returnvalue (>= (Variables|/Script/WeaponSystem_Team7.Ammo|GetCurrentAmmo _ammo) (Variables|/Script/WeaponSystem_Team7.Fire|GetBurstCount (Variables|Default|GetFire))))
    (Class|Fire|OnFire (Variables|Default|GetFire) (Utilities|Array|MakeArray (Variables|Default|GetFireMode) (Variables|Default|GetSFX) (Variables|Default|GetVFX) (Variables|Default|GetAmmo) (Variables|Default|GetRecoil)))))

(event EventOnReloadEvent
  (Class|Ammo|Reload (Variables|Default|GetAmmo)))

(fn ConstructionScript)