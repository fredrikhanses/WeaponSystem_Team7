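; SpiffeWeapon7_BP is a zoomable first-person gun Blueprint assembled from modular components.
; Fire events pass the fire mode, ammo, VFX, SFX and recoil parts to the Fire component.
; BeginPlay links recoil to the player pawn and toggles a blue gun skin through SkinToggle.
; Zoom events call the Zoom component with the supplied camera as a scoped weapon with magnification.
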(event EventOnFireEvent
  (Class|Fire|OnFire (Variables|Default|GetFire) (Utilities|Array|MakeArray (Variables|Default|GetFireMode) (Variables|Default|GetAmmo) (Variables|Default|GetVFX) (Variables|Default|GetSFX) (Variables|Default|GetRecoil))))

(event EventBeginPlay
  (bind _skintoggle (Variables|Default|GetSkinToggle))
  (Class|Recoil|SetPawn (Variables|Default|GetRecoil) (Game|Player|GetPlayerPawn 0))
  (Class|SkinToggle|SetMaterial _skintoggle "/Game/Team7_Content/Materials/M_FPGun_Blue.M_FPGun_Blue")
  (Class|SkinToggle|Toggle _skintoggle))

(event EventOnZoomEvent
  (params (Camera :type Camera%20Component%20Object%20Reference))
  (Class|Zoom|ZoomToggle (Variables|Default|GetZoom) Camera 4.0 true))

(fn ConstructionScript)