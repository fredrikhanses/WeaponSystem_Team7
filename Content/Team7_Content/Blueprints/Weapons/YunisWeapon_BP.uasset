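; Yunis's weapon Blueprint, built from components for firing, ammo, recoil and material switching, with SFX and VFX passed into each shot.
; The fire event turns on autofire, then fires and toggles a Chrome skin only if ammo passes its check and covers the burst count.
; Release stops autofire and reload delegates to Ammo.
; BeginPlay registers Ammo, binds Recoil to player 0's pawn and toggles the initial material; the zoom event is empty.
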(event Custom|YunisZoom
  (params (Camera :type Camera%20Component%20Object%20Reference)))

(event EventOnFireEvent
  (bind _skintoggle (Variables|Default|GetSkinToggle))
  (bind _returnvalue (Class|Ammo|CheckAmmo (Variables|Default|GetAmmo)))
  (Variables|/Script/WeaponSystem_Team7.Fire|SetbAutofire (Variables|Default|GetFire) true)
  (if (and _returnvalue (>= (Variables|/Script/WeaponSystem_Team7.Ammo|GetCurrentAmmo (Variables|Default|GetAmmo)) (Variables|/Script/WeaponSystem_Team7.Fire|GetBurstCount (Variables|Default|GetFire))))
    (Class|Fire|OnFire (Variables|Default|GetFire) (Utilities|Array|MakeArray (Variables|Default|GetFireMode) (Variables|Default|GetSFX) (Variables|Default|GetVFX) (Variables|Default|GetAmmo) (Variables|Default|GetRecoil)))
    (Class|SkinToggle|SetMaterial _skintoggle "/DatasmithContent/Materials/FBXImporter/VRED/Chrome.Chrome")
    (Class|SkinToggle|Toggle _skintoggle)))

(event EventOnReleaseEvent
  (Variables|/Script/WeaponSystem_Team7.Fire|SetbAutofire (Variables|Default|GetFire) false))

(event EventOnReloadEvent
  (Class|Ammo|Reload (Variables|Default|GetAmmo)))

(event EventBeginPlay
  (bind _skintoggle (Variables|Default|GetSkinToggle))
  (Class|Weapon|SetAmmoComponent (Variables|Default|GetAmmo))
  (Class|Recoil|SetPawn (Variables|Default|GetRecoil) (Game|Player|GetPlayerPawn 0))
  (Class|SkinToggle|SetMaterial _skintoggle "/Engine/EditorMaterials/Cloth/CameraLitDoubleSided.CameraLitDoubleSided")
  (Class|SkinToggle|Toggle _skintoggle))

(fn ConstructionScript)